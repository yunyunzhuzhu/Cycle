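; Volumetric cloud actor that follows the player horizontally and simulates an optional day cycle.
; Time on a 0–2400 clock rotates an arrow and directional light, feeding the sun vector to the box's dynamic cloud material.
; Curves sampled by time, mirrored around noon, drive color and lighting, while coverage, density, height and speed variables shape the clouds.
; The construction script applies this in editor; Tick refreshes it and periodically recaptures the skylight.
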(event EventBeginPlay
  ;[1 0.5944 0] Create Material Instance Reference
  (bind _returnvalue (Rendering|Material|CreateDynamicMaterialInstance (Variables|Default|GetBox) 0 (Variables|CloudAttribute|GetMatRef) :!class /Script/Engine.PrimitiveComponent))
  (Variables|Default|SetMatInsRef _returnvalue))

(event EventTick
  (params (DeltaSeconds :type Float%20%28single-precision%29))
  (bind _returnvalue (Game|Player|GetPlayerPawn 0))
  (bind _returnvalue_2 (Transformation|GetActorLocation _returnvalue))
  (bind (_x _y) (Math|Vector|BreakVector _returnvalue_2))
  (Utilities|FlowControl|Sequence
    (:then_0
      ;[1 1 1] Move Cloud along player's location
      (Utilities|IsValid _returnvalue
        (:Is%20Valid
          (Transformation|SetWorldLocation (Variables|Default|GetDefaultSceneRoot) (Math|Vector|MakeVector _x _y (.Z (Math|Vector|BreakVector (Transformation|GetWorldLocation (Variables|Default|GetDefaultSceneRoot))))) false false))
        (:Is%20Not%20Valid
          (Development|PrintString "Please Play with Character"))))
    (:then_1
      ;[0.9556 0.1475 1] Simulate sun direction by time
      (if (Variables|Time&SunAttribute|GetTimeOfDay)
        (Variables|Time&SunAttribute|SetTime (Math|Float|SelectFloat 2.4e+03 (Math|Float|SelectFloat 0.0 (+ (Variables|Time&SunAttribute|GetTime) (/ (* (/ DeltaSeconds 6e+01) 2.4e+03) (Variables|Time&SunAttribute|GetDay%20Length))) (> (+ (Variables|Time&SunAttribute|GetTime) (/ (* (/ DeltaSeconds 6e+01) 2.4e+03) (Variables|Time&SunAttribute|GetDay%20Length))) 2.4e+03)) (< (+ (Variables|Time&SunAttribute|GetTime) (/ (* (/ DeltaSeconds 6e+01) 2.4e+03) (Variables|Time&SunAttribute|GetDay%20Length))) 0.0))))
      (CallFunction|SetSunDirectionbyTime))
    (:then_2
      ;[1 1 1] Set Material's parameter from curves and public variable
      (CallFunction|SetMaterialVariable))
    (:then_3
      ;[0.548 1 0.1557] Recapture skylight
      (if (>= (Variables|Default|GetframeCount) (Variables|Default|GetskyRecapEvery))
        (Class|SkyLightComponent|RecaptureSky (Variables|/Script/Engine.SkyLight|GetLightComponent (Variables|Default|GetskyLight)))
        (Variables|Default|SetframeCount 0)
        (else
          (Math|Integer|IncrementInt (Variables|Default|GetframeCount)))))))

(fn ConstructionScript
  ;[0 0.9778 1] Create Material Instance Reference
  (bind _returnvalue (Rendering|Material|CreateDynamicMaterialInstance (Variables|Default|Getbox) 0 (Variables|CloudAttribute|GetMatRef) :!class /Script/Engine.PrimitiveComponent))
  (Variables|Default|SetMatInsRef _returnvalue)
  (CallFunction|SetSunDirectionbyTime) ; Set sun direction in Material's parameter and Directional Light by time
  ;[1 1 1] Set Material's parameter from curves and public variable
  (CallFunction|SetMaterialVariable)
  ;[0.8642 0.3444 1] Set Material to Box(Static mesh)
  (Rendering|Material|SetMaterial (Variables|Default|GetBox) 0 (Variables|Default|GetMatInsRef)))

(fn SetSunDirectionbyTime
  (bind _sun_angle (Variables|Time&SunAttribute|GetSun%20Angle))
  (bind _sun_inclination (Variables|Time&SunAttribute|GetSun%20Inclination))
  (bind _time (Variables|Time&SunAttribute|GetTime))
  (bind _returnvalue (Math|Rotator|MakeRotator 0.0 0.0 _sun_inclination))
  (bind _returnvalue_2 (Math|Float|MapRangeUnclamped _time 0.0 2.4e+03 0.0 3.6e+02))
  (bind _x (Math|Rotator|GetAxes _returnvalue))
  (bind _returnvalue_3 (+ _returnvalue_2 9e+01))
  (bind _returnvalue_4 (Math|Rotator|MakeRotator 0.0 _returnvalue_3 _sun_angle))
  (bind _returnvalue_5 (Math|Vector|RotateVector _x _returnvalue_4))
  (bind _returnvalue_6 (Math|Conversions|RotationFromXVector _returnvalue_5))
  ;[0.3122 1 0.9801] Set sun rotation value to arrow component
  (Transformation|SetWorldRotation (Variables|Default|GetArrow) _returnvalue_6 false false)
  ;[0.7448 0.3501 1] Pass Arrow Rotation(Sun Rotation) to Material as LightVector
  (Rendering|Material|SetVectorParameterValue (Variables|Default|GetMatInsRef) "LightVector" (Math|Conversions|ToLinearColor(Vector) (Math|Vector|GetForwardVector (Variables|Default|GetArrow))) :!class /Script/Engine.MaterialInstanceDynamic)
  ;[1 1 1] Set Directional light rotation
  (Transformation|SetWorldRotation (Variables|/Script/Engine.Light|GetLightComponent (Variables|Default|GetDirection%20Light)) _returnvalue_6 false false))

(fn SetMaterialVariable
  (bind _time (Variables|Time&SunAttribute|GetTime))
  (bind _matinsref (Variables|Default|GetMatInsRef))
  (bind _coverage (Variables|CloudAttribute|GetCoverage))
  (bind _returnvalue (< _time 1.2e+03))
  (bind _returnvalue_2 (Math|Float|MapRangeUnclamped _time 0.0 1.2e+03 0.0 1.0))
  (bind _returnvalue_3 (Math|Float|MapRangeUnclamped _time 1.2e+03 2.4e+03 1.0 0.0))
  (bind _returnvalue_4 (Math|Float|SelectFloat _returnvalue_2 _returnvalue_3 _returnvalue))
  ;[1 0.9083 0.4078] Set material's parameter by curves
  (Rendering|Material|SetVectorParameterValue _matinsref "CloudBaseColor" (Math|Curves|GetLinearColorValue (Variables|Curve|GetCloudBaseColor) _returnvalue_4) :!class /Script/Engine.MaterialInstanceDynamic)
  (Rendering|Material|SetVectorParameterValue _matinsref "CloudTopColor" (Math|Curves|GetLinearColorValue (Variables|Curve|GetCloudTopColor) _returnvalue_4) :!class /Script/Engine.MaterialInstanceDynamic)
  (Rendering|Material|SetVectorParameterValue _matinsref "Sun Color" (Math|Curves|GetLinearColorValue (Variables|Curve|GetLightColor) _returnvalue_4) :!class /Script/Engine.MaterialInstanceDynamic)
  (Rendering|Material|SetScalarParameterValue _matinsref "AmbientScalar" (Math|Curves|GetFloatValue (Variables|Curve|GetAmbientScalar) _returnvalue_4) :!class /Script/Engine.MaterialInstanceDynamic)
  (Rendering|Material|SetScalarParameterValue _matinsref "LightScalar" (* (Math|Curves|GetFloatValue (Variables|Curve|GetLightScalar) _returnvalue_4) (Variables|Time&SunAttribute|GetSunIntensity)) :!class /Script/Engine.MaterialInstanceDynamic)
  (Utilities|FlowControl|Sequence
    (:then_0
      ;[0.6505 1 0.481] Set Scalar parameter from public variable
      (Rendering|Material|SetScalarParameterValue _matinsref "Density" (Variables|CloudAttribute|GetDensity) :!class /Script/Engine.MaterialInstanceDynamic)
      (Rendering|Material|SetScalarParameterValue _matinsref "HeightOffset" (+ (- 0.5 (Math|Float|MapRangeClamped (Variables|CloudAttribute|GetHeightOffset) 0.0 1.0 1.1 1.25)) 0.91) :!class /Script/Engine.MaterialInstanceDynamic)
      (Rendering|Material|SetScalarParameterValue _matinsref "Coverage" (Math|Curves|GetFloatValue (Variables|Curve|GetCoverageBias) _coverage) :!class /Script/Engine.MaterialInstanceDynamic)
      (Rendering|Material|SetScalarParameterValue _matinsref "DetailStrength" (Math|Curves|GetFloatValue (Variables|Curve|GetDetailStrength) _coverage) :!class /Script/Engine.MaterialInstanceDynamic))
    (:then_1
      ;[0.4996 1 0.384] Set Vector parameter from public variable
      (Rendering|Material|SetVectorParameterValue _matinsref "BaseTranslation" (Math|Conversions|ToLinearColor(Vector) (Math|Vector|MakeVector (/ (Variables|CloudAttribute|GetSpeed) 1e+02) 0.0 0.0)) :!class /Script/Engine.MaterialInstanceDynamic))))