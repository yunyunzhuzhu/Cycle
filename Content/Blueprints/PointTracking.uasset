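; Actor that visualizes tracked points received over OSC as Niagara components, one per OSC address.
; Each message creates or moves that address's component, placing it relative to the actor by scaling two float values along ExtentA and ExtentB, and refreshes its timestamp.
; Tick destroys and forgets any point not updated within Lifetime seconds.
; A debug PrintString shows incoming float data.
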(event OnOscReceived(OscReceiver)
  (params (Address :type Name%20%28by%20ref%29 :default "None") (Data :type Array%20of%20Osc%20Data%20Elem%20Struct%20Structures) (SenderIp :type String))
  (bind (_output _value) (Class|OscFunctionLibrary|PopFloat Data))
  (if (.ReturnValue (Utilities|Map|Find (Variables|Default|GetActivePoints) Address))
    _
    (else
      (bind _returnvalue (AddComponent|AddNiagaraComponent false))
      (Utilities|Map|Add (Variables|Default|GetActivePoints) Address _returnvalue)))
  (Utilities|Map|Add (Variables|Default|GetPointTimes) Address (Math|DateTime|Now))
  (Transformation|SetRelativeTransform (.Value (Utilities|Map|Find (Variables|Default|GetActivePoints) Address)) (Math|Conversions|ToTransform(Vector) (+ (* (Variables|Default|GetExtentB) (.Value (Class|OscFunctionLibrary|PopFloat _output))) (* (Variables|Default|GetExtentA) _value))) false false)
  (Development|PrintString (Utilities|String|ToString(Float) _value)))

(event EventTick
  (params (DeltaSeconds :type Float%20%28single-precision%29))
  (bind _pointtimes (Variables|Default|GetPointTimes))
  (bind _activepoints (Variables|Default|GetActivePoints))
  (bind _keys (Utilities|Map|Keys _pointtimes))
  (for _array_element _keys
    (if (> (Math|DateTime|Now) (+ (.Value (Utilities|Map|Find _pointtimes _array_element)) (Math|Timespan|FromSeconds (Variables|Default|Getlifetime))))
      (Components|DestroyComponent (.Value (Utilities|Map|Find _activepoints _array_element)))
      (Utilities|Map|Remove _activepoints _array_element)
      (Utilities|Map|Remove (Variables|Default|GetPointTimes) _array_element))))

(fn ConstructionScript)