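; MultiCamera is a multi-view capture actor with left, right, front and hero scene captures.
; Its construction script hides the HiddenActors list from the left, right and front captures, and makes the hero capture show only those actors, separating them from the surroundings.
; An unconnected Event Graph chain would stack the four planes' materials vertically into one render target, but it never runs, and Tick is empty.
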(event EventBeginPlay)

(event Collision|EventActorBeginOverlap
  (params (OtherActor :type Actor%20Object%20Reference)))

(event EventTick
  (params (DeltaSeconds :type Float%20%28single-precision%29)))

(fn ConstructionScript
  (bind _captureleft (Variables|Default|GetCaptureLeft))
  (bind _capturehero (Variables|Default|GetCaptureHero))
  (bind _captureright (Variables|Default|GetCaptureRight))
  (bind _capturefront (Variables|Default|GetCaptureFront))
  (Variables|/Script/Engine.SceneCaptureComponent|SetPrimitiveRenderMode _captureleft "PRM_RenderScenePrimitives")
  (Variables|/Script/Engine.SceneCaptureComponent|SetPrimitiveRenderMode _captureright "PRM_RenderScenePrimitives")
  (Variables|/Script/Engine.SceneCaptureComponent|SetPrimitiveRenderMode _capturefront "PRM_RenderScenePrimitives")
  (Variables|/Script/Engine.SceneCaptureComponent|SetHiddenActors _captureleft (Variables|Default|GetHiddenActors))
  (Variables|/Script/Engine.SceneCaptureComponent|SetHiddenActors _captureright (Variables|Default|GetHiddenActors))
  (Variables|/Script/Engine.SceneCaptureComponent|SetHiddenActors _capturefront (Variables|Default|GetHiddenActors))
  (Variables|/Script/Engine.SceneCaptureComponent|SetPrimitiveRenderMode _capturehero "PRM_UseShowOnlyList")
  (for _array_element (Variables|Default|GetHiddenActors)
    (Rendering|SceneCapture|ShowOnlyActorComponents _capturehero _array_element)))