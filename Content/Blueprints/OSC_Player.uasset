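; OSC_Player is a Blueprint that lets incoming OSC messages control playback of a referenced sequence.
; Its OscReceiverComponent compares each received address against play and stop commands.
; "/play" starts the Sequencer's player, then jumps it to -30 seconds.
; "/stop" jumps to that same time before stopping, and other addresses are ignored.
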(event OnOscReceived(OscReceiverComponent)
  (params (Address :type Name%20%28by%20ref%29 :default "None") (Data :type Array%20of%20Osc%20Data%20Elem%20Struct%20Structures) (SenderIp :type String))
  (bind _sequencer (Variables|Default|GetSequencer))
  (bind _sequencer_2 (Variables|Default|GetSequencer))
  (bind _sequenceplayer (Variables|/Script/LevelSequence.LevelSequenceActor|GetSequencePlayer _sequencer_2))
  (if (Utilities|Enum|Equal(Enum) (Utilities|String|ToString(Name) Address) "/play")
    (Sequencer|Player|Play _sequenceplayer :!class /Script/MovieScene.MovieSceneSequencePlayer)
    (Class|MovieSceneSequencePlayer|JumptoSeconds _sequenceplayer -3e+01)
    (elif (Utilities|Enum|Equal(Enum) (Utilities|String|ToString(Name) Address) "/stop")
      (Class|MovieSceneSequencePlayer|JumptoSeconds (Variables|/Script/LevelSequence.LevelSequenceActor|GetSequencePlayer _sequencer) -3e+01)
      (Sequencer|Player|Stop (Variables|/Script/LevelSequence.LevelSequenceActor|GetSequencePlayer _sequencer) :!class /Script/MovieScene.MovieSceneSequencePlayer))))

(event EventBeginPlay)

(event Collision|EventActorBeginOverlap
  (params (OtherActor :type Actor%20Object%20Reference)))

(event EventTick
  (params (DeltaSeconds :type Float%20%28single-precision%29)))

(fn ConstructionScript)